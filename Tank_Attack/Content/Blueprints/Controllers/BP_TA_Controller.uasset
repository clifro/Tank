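; Player controller that drives a tank indirectly through a second controller reference, NewVar, using mouse and keyboard input.
; Left click traces under the cursor on the Visibility channel and passes the hit location through SetTarget to that controller's Dest.
; Space calls ServerFire, while the Server_fire event casts that controller's pawn to BP_Tank and calls Fire.
; The Possess event is empty.
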(event `Key|LeftMouseButton`
  (params (Key :type "Key Structure"))
  (bind (_hitresult _returnvalue) (`self.GetHitResultUnderCursorByChannel` "TraceTypeQuery1"))
  (:`Pressed`
    (if _returnvalue
      (`self.SetTarget` (`.Location` (`GameplayStatics.BreakHitResult` _hitresult))))))

(event `SetTarget`
  (params (Target :type "Vector Structure"))
  (bind _newvar (`self.NewVar`))
  (`/Engine/EditorBlueprintResources/StandardMacros.IsValid` _newvar
    (:`Is Valid`
      (set `/Game/Blueprints/Controllers/BP_TA_AI_Controller.dest` Target _newvar))))

(event `Server_fire`
  (bind _asbp_tank (cast `/Game/Blueprints/Characters/BP_Tank` (`self.K2_GetPawn` (`self.NewVar`))))
  (`/Game/Blueprints/Characters/BP_Tank.Fire` _asbp_tank))

(event `Key|SpaceBar`
  (params (Key :type "Key Structure"))
  (:`Pressed`
    (`self.Server_fire`)))

(event `self.ReceivePossess`
  (params (PossessedPawn :type "Pawn Object Reference")))

(fn `UserConstructionScript`)