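; AI controller for tanks that holds each possessed pawn at its starting spot and handles its death and respawn.
; Possess stores the pawn's location as Dest, and Tick issues a move to it every frame.
; Respawn registers the kill under the instigating player's name in BP_GS, destroys the old pawn, then spawns and possesses a new BP_Tank at a randomized X position.
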(event `self.ReceiveBeginPlay`)

(event `self.ReceiveTick`
  (params (DeltaSeconds :type "Float (single-precision)"))
  (`self.MoveToLocation` (`self.dest`) -1.0 true true false true null))

(event `self.ReceiveUnPossess`
  (params (UnpossessedPawn :type "Pawn Object Reference")))

(event `self.ReceivePossess`
  (params (PossessedPawn :type "Pawn Object Reference"))
  (set `self.dest` (`self.K2_GetActorLocation` (`self.K2_GetPawn`))))

(fn `Respawn`
  (params (Instigator :type "Actor Object Reference"))
  (locals (NewLocalVar :type "Pawn Object Reference"))
  (`/Game/GameModes/BP_GS.RegisterKill` (cast `/Game/GameModes/BP_GS` (`GameplayStatics.GetGameState`) :!pure true) (`/Game/GameModes/BP_PlayerState.PlayerName` (cast `/Game/GameModes/BP_PlayerState` (`Controller.PlayerState` (cast `PlayerController` (`self.GetOwner` Instigator) :!pure true)) :!pure true)))
  (set `local.NewLocalVar` (`self.K2_GetPawn`))
  (`self.UnPossess`)
  (`self.K2_DestroyActor` (`local.NewLocalVar`))
  (bind _returnvalue (`|SpawnActorFromClass` "/Game/Blueprints/Characters/BP_Tank.BP_Tank_C" (`KismetMathLibrary.MakeTransform` (`KismetMathLibrary.MakeVector` (`KismetMathLibrary.RandomFloatInRange` -1200.0 -2000.0) 0.0 30.0)) "AlwaysSpawn" "OverrideRootScale" (`self.GetOwner` self) null))
  (`self.Possess` _returnvalue))

(fn `UserConstructionScript`)