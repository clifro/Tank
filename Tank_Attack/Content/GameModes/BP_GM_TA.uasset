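; BP_GM_TA is a game mode that names and registers each player on login.
; PostLogin casts the new player's PlayerState to BP_PlayerState and sets its PlayerName to "Player_" plus an incrementing Id counter.
; It then passes that name to RegisterKill on the BP_GS game state.
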(event `self.ReceiveBeginPlay`)

(event `self.K2_PostLogin`
  (params (NewPlayer :type "PlayerController Object Reference"))
  (bind _asbp_player_state (cast `/Game/GameModes/BP_PlayerState` (`Controller.PlayerState` NewPlayer)))
  (bind _output_get (set `/Game/GameModes/BP_PlayerState.PlayerName` (`KismetStringLibrary.Conv_StringToName` (`KismetStringLibrary.Concat_StrStr` "Player_" (`KismetStringLibrary.Conv_IntToString` (`self.id`)))) _asbp_player_state))
  (`/Engine/EditorBlueprintResources/StandardMacros.IncrementInt` (`self.id`)
    (:`  `
      (bind _asbp_gs (cast `/Game/GameModes/BP_GS` (`GameplayStatics.GetGameState`)))
      (`/Game/GameModes/BP_GS.RegisterKill` _asbp_gs _output_get))))

(fn `UserConstructionScript`)