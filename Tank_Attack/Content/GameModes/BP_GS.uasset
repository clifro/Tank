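; Game state Blueprint that shows player scores on screen through a WB_Scores widget.
; On BeginPlay, only the Remote authority branch creates the widget, stores it and adds it to the viewport.
; UpdateScoreUI checks that the widget is valid, then passes each PlayerScores entry's ID and score to it.
; ShowScoreOnUI does the same for a supplied score array, without the validity check.
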(event `self.ReceiveBeginPlay`
  (`parent.ReceiveBeginPlay`)
  (`/Engine/EditorBlueprintResources/ActorMacros.Switch Has Authority`
    (:`Remote`
      (bind _returnvalue (`|CreateWidget` "/Game/Widgets/WB_Scores.WB_Scores_C"))
      (set `self.ScoreUIRef` _returnvalue)
      (`UserWidget.AddToViewport` _returnvalue 0))))

(event `self.UpdateScoreUI`
  (`/Engine/EditorBlueprintResources/StandardMacros.IsValid` (`self.ScoreUIRef`)
    (:`Is Valid`
      (for _array_element (`self.PlayerScores`)
        (bind (_playerid _score) (break `ScoreData` _array_element))
        (`/Game/Widgets/WB_Scores.ShowScore` (`self.ScoreUIRef`) _playerid _score)))))

(fn `ShowScoreOnUI`
  (params (Scores :type "Array of ScoreData Structure"))
  (for _array_element Scores
    (bind (_playerid _score) (break `ScoreData` _array_element))
    (`/Game/Widgets/WB_Scores.ShowScore` (`self.ScoreUIRef`) _playerid _score)))

(fn `UserConstructionScript`)